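; Player shooter character Blueprint that plays an intro sound outside the main menu and performs melee takedowns on other shooter characters.
; The TakeDown input, gated by CanTakeDown, line-traces a short distance forward and calls Takedown and GetKIlled on the BP_ShooterCharacter hit.
; Movement is disabled and IsKilling set during a brief delay, then walking resumes; CanTakeDown is not reset here.
; Unconnected nodes for head-socket camera attachment and repositioning never run.
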(event EventBeginPlay
  (|CallParentFunction)
  (bind _returnvalue (Game|GetCurrentLevelName true))
  (if (Utilities|Enum|NotEqual(Enum) _returnvalue "MainMenu")
    (Audio|PlaySoundatLocation "/Game/AssetPacks/GameDevTV/VoiceOvers/Intro.Intro" (Transformation|GetActorLocation) "0, 0, 0" 4.0 1.0 0.0 0 0 0)))

(event Collision|EventActorBeginOverlap
  (params (OtherActor :type Actor%20Object%20Reference))
  (|CallParentFunction OtherActor) ; This node is disabled and will not be called.\nDrag off pins to build functionality.
)

(event EventTick
  (params (DeltaSeconds :type Float%20%28single-precision%29))
  (|CallParentFunction DeltaSeconds) ; This node is disabled and will not be called.\nDrag off pins to build functionality.
)

(event Input|ActionEvents|InputActionTakeDown
  (params (Key :type Key%20Structure :default "None"))
  (bind _returnvalue (Transformation|GetActorLocation))
  (:Pressed
    (if (Variables|Default|GetcanTakeDown)
      (bind (_outhit _returnvalue_2) (Collision|LineTraceByChannel _returnvalue (+ _returnvalue (* (Transformation|GetActorForwardVector) 2.5e+02)) "TraceTypeQuery1" false 0 "None"))
      (if _returnvalue_2
        (bind _asshooter_character (Utilities|Casting|CastToShooterCharacter (.HitActor (Collision|BreakHitResult _outhit))))
        (Variables|Default|Settakedown_target _asshooter_character)
        (Pawn|Components|CharacterMovement|DisableMovement (Variables|Character|GetCharacterMovement))
        (Variables|Default|SetcanTakeDown false)
        (Variables|/Game/BP_ShooterCharacter.BP_ShooterCharacter_C|SetIsKilling self true)
        (bind _asbp_shooter_character (Utilities|Casting|CastToBP_ShooterCharacter (Variables|Default|Gettakedown_target)))
        (Default|Takedown _asbp_shooter_character)
        (Class|ShooterCharacter|GetKIlled _asbp_shooter_character)
        (Utilities|FlowControl|Delay 0.6)
        (Variables|Default|SetIsKilling false)
        (Pawn|Components|CharacterMovement|SetMovementMode (Variables|Character|GetCharacterMovement) "MOVE_Walking" 0)
        (Transformation|AttachComponentToComponent (Variables|Default|GetSpringArm) 0 "None" "KeepRelative" "KeepRelative" "KeepRelative" true)))))

(fn ConstructionScript
  (|CallParentFunction))